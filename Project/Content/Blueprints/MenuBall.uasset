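; MenuBall is a physics-driven sphere actor that moves at a constant speed, by its name for the menu.
; On BeginPlay a random integer picks its material, either Sun or Moon.
; Every Tick it normalizes the sphere's linear velocity and rescales it by Speed, so physics changes its direction while the speed stays fixed.
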(event `self.ReceiveBeginPlay`
  (bind _sphere (`self.Sphere`))
  (`/Engine/EditorBlueprintResources/StandardMacros.CompareInt` (`KismetMathLibrary.RandomIntegerInRange` 0 10) 5
    (:`>`
      (`PrimitiveComponent.SetMaterial` _sphere 0 (`self.moon`) :!label _label))
    (:`==`
      (goto _label))
    (:`<`
      (`PrimitiveComponent.SetMaterial` _sphere 0 (`self.sun`)))))

(event `self.ReceiveTick`
  (params (DeltaSeconds :type "Float (single-precision)"))
  (bind _sphere (`self.Sphere`))
  (bind _returnvalue (`PrimitiveComponent.GetPhysicsLinearVelocity` _sphere "None"))
  (`PrimitiveComponent.SetPhysicsLinearVelocity` _sphere (* (`KismetMathLibrary.Normal` _returnvalue) (`self.speed`)) false "None"))

(fn `UserConstructionScript`)