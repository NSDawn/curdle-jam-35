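; Pinball-style player controls that drive left and right flippers and a launcher, and keep a points total.
; Key presses set flip and launch flags, with UseLJIKeys choosing between J/I/L and A/W/D layouts.
; Tick interpolates each part toward its end or rest transform, clearing its flag on arrival so it returns automatically.
; AddPoints clamps the total at zero and broadcasts the score change.
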(event `self.ReceiveBeginPlay`
  (bind _mat (`self.mat`))
  (set `self.rightPad_OriginalRot` (`SceneComponent.K2_GetComponentRotation` (`self.RightFlipperParent`)))
  (set `self.leftPad_OriginalRot` (`SceneComponent.K2_GetComponentRotation` (`self.LeftFlipperParent`)))
  (bind _output_get (set `self.launch_OriginalPos` (`SceneComponent.K2_GetComponentLocation` (`self.Launcher`))))
  (set `self.launch_EndPos` (+ _output_get (`self.launch_EndPos`)))
  (`PrimitiveComponent.SetMaterial` (`self.RightFlipper`) 0 _mat)
  (`PrimitiveComponent.SetMaterial` (`self.LeftFlipper`) 0 _mat)
  (`PrimitiveComponent.SetMaterial` (`self.Launcher`) 0 _mat))

(event `Key|I` :consume false
  (params (Key :type "Key Structure"))
  (:`Pressed`
    (if (`self.useLJIKeys`)
      (set `self.isLaunch` true :!label _label))))

(event `Key|J` :consume false
  (params (Key :type "Key Structure"))
  (:`Pressed`
    (if (`self.useLJIKeys`)
      (set `self.leftFlipping` true :!label _label_2))))

(event `Key|L` :consume false
  (params (Key :type "Key Structure"))
  (:`Pressed`
    (if (`self.useLJIKeys`)
      (set `self.rightFlipping` true :!label _label_3))))

(event `Key|W` :consume false
  (params (Key :type "Key Structure"))
  (:`Pressed`
    (if (not (`self.useLJIKeys`))
      (goto _label))))

(event `Key|A` :consume false
  (params (Key :type "Key Structure"))
  (:`Pressed`
    (if (not (`self.useLJIKeys`))
      (goto _label_2))))

(event `Key|D` :consume false
  (params (Key :type "Key Structure"))
  (:`Pressed`
    (if (not (`self.useLJIKeys`))
      (goto _label_3))))

(event `self.ReceiveTick`
  (params (DeltaSeconds :type "Float (single-precision)"))
  (bind _returnvalue (`SceneComponent.K2_GetComponentRotation` (`self.LeftFlipperParent`)))
  (bind _returnvalue_2 (`SceneComponent.K2_GetComponentRotation` (`self.RightFlipperParent`)))
  (bind _returnvalue_3 (`SceneComponent.K2_GetComponentLocation` (`self.Launcher`)))
  (bind _returnvalue_4 (select `bool` (`self.leftFlipping`) :`false` (`self.leftPad_OriginalRot`) :`true` (`self.leftPad_EndRot`)))
  (bind _returnvalue_5 (select `bool` (`self.rightFlipping`) :`false` (`self.rightPad_OriginalRot`) :`true` (`self.rightPad_EndRot`)))
  (bind _returnvalue_6 (select `bool` (`self.isLaunch`) :`false` (`self.launch_OriginalPos`) :`true` (`self.launch_EndPos`)))
  (`SceneComponent.K2_SetRelativeRotation` (`self.LeftFlipperParent`) (`KismetMathLibrary.RInterpTo` _returnvalue _returnvalue_4 DeltaSeconds (`self.rotSpeed`)) false false)
  (`/Engine/EditorBlueprintResources/StandardMacros.CompareFloat` (`KismetMathLibrary.Abs` (- (`KismetMathLibrary.Dot_VectorVector` (`KismetMathLibrary.GetForwardVector` _returnvalue) (`KismetMathLibrary.GetForwardVector` _returnvalue_4)) 1.0)) 0.001
    (:`>`
      _)
    (:`==`
      (set `self.leftFlipping` false :!label _label_4))
    (:`<`
      (goto _label_4)))
  (`SceneComponent.K2_SetRelativeRotation` (`self.RightFlipperParent`) (`KismetMathLibrary.RInterpTo` _returnvalue_2 _returnvalue_5 DeltaSeconds (`self.rotSpeed`)) false false)
  (`/Engine/EditorBlueprintResources/StandardMacros.CompareFloat` (`KismetMathLibrary.Abs` (- (`KismetMathLibrary.Dot_VectorVector` (`KismetMathLibrary.GetForwardVector` _returnvalue_2) (`KismetMathLibrary.GetForwardVector` _returnvalue_5)) 1.0)) 0.001
    (:`>`
      _)
    (:`==`
      (set `self.rightFlipping` false :!label _label_5))
    (:`<`
      (goto _label_5)))
  (`SceneComponent.K2_SetWorldLocation` (`self.Launcher`) (`KismetMathLibrary.VInterpTo` _returnvalue_3 _returnvalue_6 DeltaSeconds (`self.launchSpeed`)) false false)
  (`/Engine/EditorBlueprintResources/StandardMacros.CompareFloat` (`KismetMathLibrary.Vector_Distance` _returnvalue_3 _returnvalue_6) 0.1
    (:`==`
      _)
    (:`<`
      _))
  (set `self.isLaunch` false))

(fn `AddPoints`
  (params (points :type Integer))
  (returns (newScore :type Integer))
  (bind _output_get (set `self.points` (`KismetMathLibrary.Max` (+ points (`self.points`)))))
  (`self.OnScoreIncrease` _output_get)
  (return _output_get))

(fn `UserConstructionScript`)