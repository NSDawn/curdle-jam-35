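; A pinball ball actor owned by a player, showing that player's material and tracking who gets credit.
; Hitting a player's tagged Flipper component hands ownership to that PlayerControls and recolors the ball.
; Pin hits call the pin's Hit and play the owner's sound.
; Touching a KillBox resets it to its start position, deducts the owner's points, restores the original owner and plays a fail sound.
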(event `self.ReceiveBeginPlay`
  (bind _player (`self.player`))
  (set `self.originalPos` (`self.K2_GetActorLocation`))
  (set `self.originalPlayer` _player)
  (`PrimitiveComponent.SetMaterial` (`self.Sphere`) 0 (`/Game/Blueprints/PlayerControls.mat` _player)))

(event `self.ReceiveHit`
  (params (MyComp :type "PrimitiveComponent Object Reference") (Other :type "Actor Object Reference") (OtherComp :type "PrimitiveComponent Object Reference") (bSelfMoved :type Boolean) (HitLocation :type "Vector Structure") (HitNormal :type "Vector Structure") (NormalImpulse :type "Vector Structure") (Hit :type "HitResult Structure (by ref)"))
  (bind _returnvalue (`GameplayStatics.GetObjectClass` Other))
  (if (`KismetMathLibrary.ClassIsChildOf` _returnvalue "/Game/Blueprints/Pin.Pin_C")
    (bind _aspin (cast `/Game/Blueprints/Pin` Other))
    (`/Game/Blueprints/Pin.Hit` _aspin _aspin self)
    (`GameplayStatics.SpawnSound2D` (`/Game/Blueprints/PlayerControls.hitSound` (`self.player`)) 0.2 1.0 0.0 null)
    (elif (and (`KismetMathLibrary.ClassIsChildOf` _returnvalue "/Game/Blueprints/PlayerControls.PlayerControls_C") (`ActorComponent.ComponentHasTag` OtherComp "Flipper"))
      (bind _asplayer_controls (cast `/Game/Blueprints/PlayerControls` Other))
      (bind _output_get (set `self.player` _asplayer_controls))
      (`PrimitiveComponent.SetMaterial` (`self.Sphere`) 0 (`/Game/Blueprints/PlayerControls.mat` _output_get))
      (elif (`KismetMathLibrary.ClassIsChildOf` _returnvalue "/Game/Blueprints/KillBox.KillBox_C")
        (`SceneComponent.K2_SetWorldLocation` (`self.Sphere`) (`self.originalPos`) false false)
        (`/Game/Blueprints/PlayerControls.AddPoints` (`self.player`) -10)
        (bind _output_get_2 (set `self.player` (`self.originalPlayer`)))
        (`PrimitiveComponent.SetMaterial` (`self.Sphere`) 0 (`/Game/Blueprints/PlayerControls.mat` _output_get_2))
        (`GameplayStatics.SpawnSound2D` "/Game/SFX/fail.fail" 1.0 1.0 0.0 null)))))

(fn `UserConstructionScript`)