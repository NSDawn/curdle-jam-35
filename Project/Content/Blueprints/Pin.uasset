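; Pin bumper that knocks balls away and serves as a tug-of-war scoring target for two players.
; The Hit event applies a clamped impulse away from the pin and pops the visuals' scale, which Tick eases back.
; The Hit function, debounced by a short cooldown, shifts Control toward the ball's player and awards points, multiplied for the controlling side.
; UpdateMats colors five segments to show the owner's control level, alongside a text readout.
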(event `self.ReceiveBeginPlay`
  (set `self.originalScale` (`SceneComponent.K2_GetComponentScale` (`self.Visuals`))))

(event `self.ReceiveHit`
  (params (MyComp :type "PrimitiveComponent Object Reference") (Other :type "Actor Object Reference") (OtherComp :type "PrimitiveComponent Object Reference") (bSelfMoved :type Boolean) (HitLocation :type "Vector Structure") (HitNormal :type "Vector Structure") (NormalImpulse :type "Vector Structure") (Hit :type "HitResult Structure (by ref)"))
  (`PrimitiveComponent.AddImpulse` OtherComp (`KismetMathLibrary.ClampVectorSize` (* (* (`KismetMathLibrary.Normal` (- (`SceneComponent.K2_GetComponentLocation` MyComp) (`SceneComponent.K2_GetComponentLocation` OtherComp))) (`KismetMathLibrary.VSize` NormalImpulse)) -20.0) (`self.minImpulse`) (`self.maxImpulse`)) "None" false)
  (set `self.hitAnimTimer` (`self.hitAnimDur`))
  (`SceneComponent.SetWorldScale3D` (`self.Visuals`) (`self.hitScale`)))

(event `self.ReceiveTick`
  (params (DeltaSeconds :type "Float (single-precision)"))
  (bind _hitanimtimer (`self.hitAnimTimer`))
  (set `self.lastHit` (- (`self.lastHit`) DeltaSeconds))
  (`/Engine/EditorBlueprintResources/StandardMacros.CompareFloat` _hitanimtimer
    (:`>`
      (set `self.hitAnimTimer` (- _hitanimtimer DeltaSeconds))
      (`SceneComponent.SetWorldScale3D` (`self.Visuals`) (`KismetMathLibrary.VLerp` (`self.originalScale`) (`self.hitScale`) (/ _hitanimtimer (`self.hitAnimDur`)))))))

(fn `Hit`
  (params (Pin :type "/Game/Blueprints/Pin Object Reference") (Ball :type "/Game/Blueprints/Ball Object Reference"))
  (returns (Control :type Integer))
  (bind _player (`/Game/Blueprints/Ball.player` Ball))
  (bind _control (`/Game/Blueprints/Pin.control` Pin))
  (bind _control_2 (`self.control`))
  (bind _basepoints (`self.basePoints`))
  (bind _playernum (`/Game/Blueprints/PlayerControls.playerNum` _player))
  (`/Engine/EditorBlueprintResources/StandardMacros.CompareFloat` (`self.lastHit`)
    (:`>`
      _)
    (:`==`
      (set `/Game/Blueprints/Pin.control` (`KismetMathLibrary.Clamp` (select `int` _playernum :`0` (+ _control 1) :`1` (- _control 1)) -5 5) Pin :!label _label)
      (set `self.player` (select `bool` (== _playernum (select `bool` (> (`self.control`) 0) :`false` 1)) :`false` (`self.player`) :`true` _player))
      (`self.UpdateMats`)
      (`TextRenderComponent.K2_SetText` (`self.TextRender`) (`KismetTextLibrary.Conv_IntToText` _control_2))
      (`/Game/Blueprints/PlayerControls.AddPoints` _player (select `bool` (== _playernum (select `bool` (> _control_2 0) :`false` 1)) :`false` _basepoints :`true` (* (`KismetMathLibrary.Abs_Int` _control_2) _basepoints)))
      (set `self.lastHit` 0.2))
    (:`<`
      (goto _label)))
  (return _control_2))

(fn `UpdateMats`
  (bind _2 (`self.2`))
  (bind _3 (`self.3`))
  (bind _4 (`self.4`))
  (bind _5 (`self.5`))
  (bind _1 (`self.1`))
  (bind _returnvalue (`KismetMathLibrary.Abs_Int` (`self.control`)))
  (`/Engine/EditorBlueprintResources/StandardMacros.CompareInt` _returnvalue 1
    (:`>`
      (`PrimitiveComponent.SetMaterial` _1 0 (`/Game/Blueprints/PlayerControls.mat` (`self.player`)) :!label _label))
    (:`==`
      (goto _label))
    (:`<`
      (`PrimitiveComponent.SetMaterial` _1 0 "/Engine/BasicShapes/BasicShapeMaterial.BasicShapeMaterial")))
  (`/Engine/EditorBlueprintResources/StandardMacros.CompareInt` _returnvalue 2
    (:`>`
      (`PrimitiveComponent.SetMaterial` _2 0 (`/Game/Blueprints/PlayerControls.mat` (`self.player`)) :!label _label_2))
    (:`==`
      (goto _label_2))
    (:`<`
      (`PrimitiveComponent.SetMaterial` _2 0 "/Engine/BasicShapes/BasicShapeMaterial.BasicShapeMaterial")))
  (`/Engine/EditorBlueprintResources/StandardMacros.CompareInt` _returnvalue 3
    (:`>`
      (`PrimitiveComponent.SetMaterial` _3 0 (`/Game/Blueprints/PlayerControls.mat` (`self.player`)) :!label _label_3))
    (:`==`
      (goto _label_3))
    (:`<`
      (`PrimitiveComponent.SetMaterial` _3 0 "/Engine/BasicShapes/BasicShapeMaterial.BasicShapeMaterial")))
  (`/Engine/EditorBlueprintResources/StandardMacros.CompareInt` _returnvalue 4
    (:`>`
      (`PrimitiveComponent.SetMaterial` _4 0 (`/Game/Blueprints/PlayerControls.mat` (`self.player`)) :!label _label_4))
    (:`==`
      (goto _label_4))
    (:`<`
      (`PrimitiveComponent.SetMaterial` _4 0 "/Engine/BasicShapes/BasicShapeMaterial.BasicShapeMaterial")))
  (`/Engine/EditorBlueprintResources/StandardMacros.CompareInt` _returnvalue 5
    (:`>`
      (`PrimitiveComponent.SetMaterial` _5 0 (`/Game/Blueprints/PlayerControls.mat` (`self.player`)) :!label _label_5))
    (:`==`
      (goto _label_5))
    (:`<`
      (`PrimitiveComponent.SetMaterial` _5 0 "/Engine/BasicShapes/BasicShapeMaterial.BasicShapeMaterial"))))

(fn `UserConstructionScript`)