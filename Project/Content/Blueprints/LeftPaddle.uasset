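; Left paddle actor that flips toward an end rotation when the A key is pressed, then returns by itself.
; BeginPlay caches the start rotation, and the key press sets a Flipping flag that selects the target.
; Tick interpolates toward that target with RInterpTo at RotSpeed.
; A forward-vector dot product check clears the flag once the target is nearly reached, so key release plays no part.
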(event `self.ReceiveBeginPlay`
  (set `self.startRot` (`self.K2_GetActorRotation`))
  (`KismetSystemLibrary.PrintString` "left init"))

(event `Key|A`
  (params (Key :type "Key Structure"))
  (:`Pressed`
    (set `self.flipping` true)
    (`KismetSystemLibrary.PrintString` "left shift pressed")))

(event `self.ReceiveTick`
  (params (DeltaSeconds :type "Float (single-precision)"))
  (bind _returnvalue (select `bool` (`self.flipping`) :`false` (`self.startRot`) :`true` (`self.endRot`)))
  (`self.K2_SetActorRotation` (`KismetMathLibrary.RInterpTo` (`self.K2_GetActorRotation`) _returnvalue DeltaSeconds (`self.rotSpeed`)))
  (`/Engine/EditorBlueprintResources/StandardMacros.CompareFloat` (`KismetMathLibrary.Abs` (- (`KismetMathLibrary.Dot_VectorVector` (`KismetMathLibrary.GetForwardVector` (`self.K2_GetActorRotation`)) (`KismetMathLibrary.GetForwardVector` _returnvalue)) 1.0)) 0.001
    (:`==`
      _)
    (:`<`
      _))
  (set `self.flipping` false))

(fn `UserConstructionScript`)